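; BP_Character is a top-down character Blueprint that adds camera control and a hold-to-aim input.
; The construction script sets the camera boom's length, rotation and lag toggle from variables, while the lag speed assignment is left unconnected.
; Mouse wheel input drives CameraSlide, which steps the boom length within min/max limits, and right mouse switches movement state between Aim and Run.
; CameraShakeEvent plays a world shake at the camera's location.
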(event Input|AxisEvents|InputAxisMouseWheel
  (params (AxisValue :type Float%20%28single-precision%29))
  (CallFunction|CameraSlide AxisValue))

(event Input|MouseEvents|RightMouseButton
  (params (Key :type Key%20Structure :default "None"))
  (:Pressed
    (Class|TDSCharacter|ChangeMovementState "Aim_State"))
  (:Released
    (Class|TDSCharacter|ChangeMovementState "Run_State")))

(fn ConstructionScript
  (bind _cameraboom (Variables|Default|GetCameraBoom))
  (Variables|/Script/Engine.SpringArmComponent|SetTargetArmLength _cameraboom (Variables|Camera|GetHieght))
  (Transformation|SetRelativeRotation _cameraboom (Variables|Camera|GetRotatorCamera) false false)
  (Variables|/Script/Engine.SpringArmComponent|SetbEnableCameraLag _cameraboom (Variables|Camera|GetFlow)))

(fn CameraShakeEvent
  (Camera|PlayWorldCameraShake "/Game/Blueprint/Game/BP_ShakeCamera.BP_ShakeCamera_C" (Transformation|GetWorldLocation (Variables|Default|GetTopDownCameraComponent)) 0.0 3e+01))

(fn CameraSlide
  (params (Value :type Float%20%28single-precision%29))
  (bind _cameraboom (Variables|Default|GetCameraBoom))
  (bind _heightcamerachangedistanse (Variables|Camera|GetHeightCameraChangeDistanse))
  (if (!= Value 0.0)
    (if (< Value 0.0)
      (if (> (Variables|Camera|GetHieghtCameraMax) (+ (Variables|/Script/Engine.SpringArmComponent|GetTargetArmLength _cameraboom) _heightcamerachangedistanse))
        (Variables|/Script/Engine.SpringArmComponent|SetTargetArmLength _cameraboom (+ (Variables|/Script/Engine.SpringArmComponent|GetTargetArmLength _cameraboom) _heightcamerachangedistanse)))
      (elif (< (Variables|Camera|GetHieghtCameraMin) (- (Variables|/Script/Engine.SpringArmComponent|GetTargetArmLength _cameraboom) _heightcamerachangedistanse))
        (Variables|/Script/Engine.SpringArmComponent|SetTargetArmLength _cameraboom (- (Variables|/Script/Engine.SpringArmComponent|GetTargetArmLength _cameraboom) _heightcamerachangedistanse))))))